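; BP_player is the player Blueprint, handling look, movement and grab input.
; Movement follows the control rotation's yaw only, keeping it on the horizontal plane regardless of camera pitch.
; Pressing and releasing grab calls StartGrab and ReleaseGrab on Grab, which holds the grab logic.
; Disconnected line trace and PhysicsHandle nodes for grabbing physics objects remain in the graph but never run.
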(event `InputAxis|turn`
  (params (AxisValue :type "Float (single-precision)"))
  (`self.AddControllerYawInput` AxisValue))

(event `InputAxis|look up`
  (params (AxisValue :type "Float (single-precision)"))
  (`self.AddControllerPitchInput` AxisValue))

(event `InputAxis|move forwards`
  (params (AxisValue :type "Float (single-precision)"))
  (`self.AddMovementInput` (`KismetMathLibrary.GetForwardVector` (`KismetMathLibrary.MakeRotator` 0.0 0.0 (.yaw (`self.GetControlRotation`)))) AxisValue))

(event `InputAxis|move right / left`
  (params (AxisValue :type "Float (single-precision)"))
  (`self.AddMovementInput` (`KismetMathLibrary.GetRightVector` (`KismetMathLibrary.MakeRotator` 0.0 0.0 (.yaw (`self.GetControlRotation`)))) AxisValue))

(event `InputAction|grab`
  (params (Key :type "Key Structure"))
  (bind _grab (`self.grab`))
  (:`Pressed`
    (`ActorPosition.startGrab` _grab))
  (:`Released`
    (`ActorPosition.releaseGrab` _grab)))

(event `self.ReceiveTick`
  (params (DeltaSeconds :type "Float (single-precision)")))

(fn `UserConstructionScript`)