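; BP_porte is a weight-activated door that slides vertically when a physics object enters its trigger box.
; On overlap with a simulating component, it stores the mass divided by 100 and plays the OuverturePorte timeline.
; The timeline interpolates the Door's relative Z downward by a distance proportional to that mass, so heavier objects move it further.
; Any component leaving the box reverses the timeline.
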(event `self.Box.OnComponentBeginOverlap`
  (params (OverlappedComponent :type "PrimitiveComponent Object Reference") (OtherActor :type "Actor Object Reference") (OtherComp :type "PrimitiveComponent Object Reference") (OtherBodyIndex :type Integer) (bFromSweep :type Boolean) (SweepResult :type "HitResult Structure (by ref)"))
  (if (`SceneComponent.IsSimulatingPhysics` OtherComp "None")
    (set `self.MassObject` (/ (`PrimitiveComponent.GetMass` OtherComp) 100.0))
    (bind (_direction _newtrack_0) (`Timeline|ouverture porte` :!label _label)
      (:`Update`
        (`SceneComponent.K2_SetRelativeLocation` (`self.door`) (`KismetMathLibrary.MakeVector` 0.0 45.0 (`KismetMathLibrary.Lerp` 0.0 (* (`self.MassObject`) -200.0) _newtrack_0)) false false)))))

(event `self.Box.OnComponentEndOverlap`
  (params (OverlappedComponent :type "PrimitiveComponent Object Reference") (OtherActor :type "Actor Object Reference") (OtherComp :type "PrimitiveComponent Object Reference") (OtherBodyIndex :type Integer))
  (goto _label :!via `Reverse`))

(fn `UserConstructionScript`)